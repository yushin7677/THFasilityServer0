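; Tube actor that visualizes temperature data on the STANDTUBE mesh, polling a web server every second via VaRest for nine JSON values stored in Temp.
; Each cycle redraws a render target as a color strip from DataTable rows, calls TempUpdate, and packs twelve FullTemp values into the mesh's custom primitive data.
; Tick feeds actor X scale and yaw to the mesh materials.
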(event Custom|GetFromServer
  (bind _returnvalue (Class|VaRestSubsystem|ConstructVaRestRequestExt (|VaRestSubsystem) "GET" "x_www_form_urlencoded_url"))
  (bind _output_get (Variables|Default|Setjson%20request _returnvalue))
  (Class|VaRestRequestJSON|ProcessURL _output_get "http://yushinfk.beget.tech/")
  (EventDispatchers|BindEventtoOnRequestComplete _output_get (delegate Custom|CustomEvent_0)))

(event Custom|CustomEvent_0
  (params (Request :type Va%20Rest%20Request%20JSON%20Object%20Reference))
  (bind _returnvalue (Class|VaRestRequestJSON|GetResponseContentasString Request false))
  (bind _returnvalue_2 (Class|VaRestSubsystem|ConstructVaRestJsonObject (|VaRestSubsystem)))
  (bind _output_get (Variables|Default|Setjson%20object _returnvalue_2))
  (Class|VaRestJsonObject|DecodeJson _output_get _returnvalue true)
  (Variables|Default|Settemp (Utilities|Array|MakeArray (Class|VaRestJsonObject|GetNumberField (Variables|Default|Getjson%20object) "0") (Class|VaRestJsonObject|GetNumberField (Variables|Default|Getjson%20object) "1") (Class|VaRestJsonObject|GetNumberField (Variables|Default|Getjson%20object) "2") (Class|VaRestJsonObject|GetNumberField (Variables|Default|Getjson%20object) "3") (Class|VaRestJsonObject|GetNumberField (Variables|Default|Getjson%20object) "4") (Class|VaRestJsonObject|GetNumberField (Variables|Default|Getjson%20object) "5") (Class|VaRestJsonObject|GetNumberField (Variables|Default|Getjson%20object) "6") (Class|VaRestJsonObject|GetNumberField (Variables|Default|Getjson%20object) "7") (Class|VaRestJsonObject|GetNumberField (Variables|Default|Getjson%20object) "8"))))

(event Custom|CustomEvent_1
  (bind _fulltemp (Variables|Default|GetfullTemp))
  (bind _datatable (Variables|Default|GetDataTable))
  (bind _shitrt (Variables|Default|GetShitRT))
  (CallFunction|GetfromServer)
  (Rendering|ClearRenderTarget2D _shitrt)
  (bind (_canvas _size _context) (Rendering|BeginDrawCanvastoRenderTarget _shitrt))
  (CallFunction|GetfromServer)
  (bind _outrownames (DataTable|GetDataTableRowNames _datatable))
  (for (_array_element _array_index) _outrownames
    (bind _returnvalue (Utilities|GetDataTableRow _datatable _array_element)
      (:then
        (Class|Canvas|DrawLine _canvas (Math|Vector2D|MakeVector2D (Math|Conversions|ToFloat(Integer) _array_index) 0.0) (Math|Vector2D|MakeVector2D (+ (Math|Conversions|ToFloat(Integer) _array_index) 1.0) 0.0) 1e+01 (Utilities|Struct|MakeLinearColor (.y (Utilities|Struct|Break4vector _returnvalue)) (.z (Utilities|Struct|Break4vector _returnvalue)) (.w (Utilities|Struct|Break4vector _returnvalue)) 1.0)))))
  (Rendering|EndDrawCanvastoRenderTarget _context)
  (Class|ThBody|TempUpdate 25.0 (Variables|Default|GetminTemp))
  (for _index (range 0 3)
    (Rendering|Material|SetCustomPrimitiveDataVector3 (Variables|Default|GetSTAND_TUBE) (* _index 3) (Math|Vector|MakeVector (Utilities|Array|Get(acopy) _fulltemp (+ (* _index 3) 0)) (Utilities|Array|Get(acopy) _fulltemp (+ (* _index 3) 1)) (Utilities|Array|Get(acopy) _fulltemp (+ (* _index 3) 2))))))

(event EventTick
  (params (DeltaSeconds :type Float%20%28single-precision%29))
  (Rendering|Material|SetScalarParameterValueonMaterials (Variables|Default|GetSTAND_TUBE) "Scale1" (.x (Transformation|GetActorScale3D)))
  (Rendering|Material|SetScalarParameterValueonMaterials (Variables|Default|GetSTAND_TUBE) "Rotate1" (.yaw (Transformation|GetActorRotation))))

(event EventBeginPlay
  (bind _fulltemp (Variables|Default|GetfullTemp))
  (bind _datatable (Variables|Default|GetDataTable))
  (bind _shitrt (Variables|Default|GetShitRT))
  (Utilities|Time|SetTimerbyEvent (delegate Custom|CustomEvent_1) 1.0 true)
  (Rendering|ClearRenderTarget2D _shitrt)
  (bind (_canvas _size _context) (Rendering|BeginDrawCanvastoRenderTarget _shitrt))
  (CallFunction|GetfromServer)
  (bind _outrownames (DataTable|GetDataTableRowNames _datatable))
  (for (_array_element _array_index) _outrownames
    (bind _returnvalue (Utilities|GetDataTableRow _datatable _array_element)
      (:then
        (Class|Canvas|DrawLine _canvas (Math|Vector2D|MakeVector2D (Math|Conversions|ToFloat(Integer) _array_index) 0.0) (Math|Vector2D|MakeVector2D (+ (Math|Conversions|ToFloat(Integer) _array_index) 1.0) 0.0) 1e+01 (Utilities|Struct|MakeLinearColor (.y (Utilities|Struct|Break4vector _returnvalue)) (.z (Utilities|Struct|Break4vector _returnvalue)) (.w (Utilities|Struct|Break4vector _returnvalue)) 1.0)))))
  (Rendering|EndDrawCanvastoRenderTarget _context)
  (Class|ThBody|TempUpdate 25.0 (Variables|Default|GetminTemp))
  (for _index (range 0 3)
    (Rendering|Material|SetCustomPrimitiveDataVector3 (Variables|Default|GetSTAND_TUBE) (* _index 3) (Math|Vector|MakeVector (Utilities|Array|Get(acopy) _fulltemp (+ (* _index 3) 0)) (Utilities|Array|Get(acopy) _fulltemp (+ (* _index 3) 1)) (Utilities|Array|Get(acopy) _fulltemp (+ (* _index 3) 2))))))

(fn ConstructionScript)