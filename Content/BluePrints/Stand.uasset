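; Stand is a Blueprint that toggles the look of its static meshes through a changemat event.
; A FlipFlop alternates each call between applying the Opas material to slot 0 and setting that slot to no material, which clears the override.
; Both branches walk all descendants of DefaultSceneRoot and cast each to StaticMeshComponent to reach the meshes.
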(event Custom|changemat
  (Utilities|FlowControl|FlipFlop
    (:A
      (for _array_element (Components|GetChildrenComponents (Variables|Default|GetDefaultSceneRoot) true)
        (bind _asstatic_mesh_component (Utilities|Casting|CastToStaticMeshComponent _array_element))
        (Rendering|Material|SetMaterial _asstatic_mesh_component 0 "/Game/Materials/opas.opas")))
    (:B
      (for _array_element_2 (Components|GetChildrenComponents (Variables|Default|GetDefaultSceneRoot) true)
        (bind _asstatic_mesh_component_2 (Utilities|Casting|CastToStaticMeshComponent _array_element_2))
        (Rendering|Material|SetMaterial _asstatic_mesh_component_2 0 0)))))

(fn ConstructionScript)